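; BP_Cuttable is a sliceable prop for the LazerEyes superpower, built on a procedural mesh.
; The construction script sets the chosen static mesh and copies it into the procedural mesh with collision.
; BeginCut slices that mesh on the given plane, capping the cut with M_Floor as a new section.
; The new half simulates physics and gets a velocity-change impulse against the plane normal.
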(event Custom|Begin%20Cut
  (params (Location :type Vector) (PlaneNormal :type Vector))
  (bind _outotherhalfprocmesh (Class|KismetProceduralMeshLibrary|SliceProceduralMesh (Variables|Default|GetProceduralMesh) Location PlaneNormal true "CreateNewSectionForCap" "/Game/CharacterBodyFX/Materials/M_Floor.M_Floor"))
  (Physics|SetSimulatePhysics _outotherhalfprocmesh true)
  (Physics|AddImpulse _outotherhalfprocmesh (* (Math|Vector|NegateVector PlaneNormal) 6e+02) "None" true))

(event EventTick
  (params (DeltaSeconds :type Float%20%28single-precision%29)))

(fn ConstructionScript
  (Components|StaticMesh|SetStaticMesh (Variables|Default|GetStaticMesh) (Variables|Default|GetStatic%20Mesh%20Comp))
  (Class|KismetProceduralMeshLibrary|CopyProceduralMeshfromStaticMeshComponent (Variables|Default|GetStaticMesh) 0 (Variables|Default|GetProceduralMesh) true))