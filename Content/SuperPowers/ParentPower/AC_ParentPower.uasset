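; Parent power component that gives its owning actor the super powers listed in PlayerSuperPowers and manages which one is active.
; On BeginPlay it adds the input mapping, creates Teleport, Telekinesis, Invisibility and Lazer Eyes components as listed, attaches them to itself and activates the selected one.
; Mind Control, Strength and Flying cases create nothing yet.
; IA_SwitchPower cycles through the stored components with wraparound, toggling each via SetAsActivePower.
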(event Input|EnhancedActionEvents|EnhancedInputActionIA_SwitchPower
  (params (ActionValue :type Boolean) (ElapsedSeconds :type Float%20%28double-precision%29) (TriggeredSeconds :type Float%20%28double-precision%29) (InputAction :type Input%20Action%20Object%20Reference :default "/Game/SuperPowers/SuperPowerInputs/Actions/IA_SwitchPower.IA_SwitchPower"))
  (:Started
    (Development|PrintString "Switching Power")
    (Utilities|FlowControl|DoOnce false :!label _label
      (:Completed
        (bind _result (Math|Integer|IncrementInt (Variables|Default|GetSelected%20Super%20Power%20Index))
          (:%20%20
            (if (> _result (Utilities|Array|LastIndex (Variables|Default|GetSuper%20Power%20Components)))
              (Variables|Default|SetSelected%20Super%20Power%20Index 0))
            (Utilities|IsValid (Variables|Default|GetCurrently%20Active%20Power)
              (:Is%20Valid
                (Default|SetasActivePower (Variables|Default|GetCurrently%20Active%20Power) false))
              (:Is%20Not%20Valid
                _))
            (bind _output_get (Variables|Default|SetCurrently%20Active%20Power (.Power%20Component (CallFunction|GetSuperPowerbyIndex (Variables|Default|GetSelected%20Super%20Power%20Index)))))
            (Variables|Default|SetActive%20Power%20Name (.Power%20Name (CallFunction|GetSuperPowerbyIndex (Variables|Default|GetSelected%20Super%20Power%20Index))))
            (Default|SetasActivePower _output_get true))))))
  (:Completed
    (goto _label Reset)))

(event EventBeginPlay
  (bind _selected_super_power_index (Variables|Default|GetSelected%20Super%20Power%20Index))
  (bind (_power_component _power_name) (CallFunction|GetSuperPowerbyIndex _selected_super_power_index))
  (Variables|Default|SetOwning%20Actor (Components|GetOwner))
  (Utilities|FlowControl|Sequence
    (:then_0
      (|AddInputMapping))
    (:then_1
      (for _array_element (Variables|Default|GetPlayer%20Super%20Powers)
        (switch Utilities|FlowControl|Switch|SwitchonE_SuperPowerType _array_element
          (:NewEnumerator0
            (Utilities|FlowControl|DoOnce false
              (:Completed
                (bind _returnvalue (Game|AddComponentbyClass (Variables|Default|GetOwning%20Actor) "/Game/SuperPowers/Teleport/SC_TeleportPower.SC_TeleportPower_C" false))
                (CallFunction|AddNewPower _returnvalue))))
          (:NewEnumerator1
            (Utilities|FlowControl|DoOnce false
              (:Completed
                (bind _returnvalue_2 (Game|AddComponentbyClass (Variables|Default|GetOwning%20Actor) "/Game/SuperPowers/Telekenisis/SC_Telekenisis.SC_Telekenisis_C" false))
                (CallFunction|AddNewPower _returnvalue_2))))
          (:NewEnumerator2
            (Utilities|FlowControl|DoOnce false))
          (:NewEnumerator3
            (Utilities|FlowControl|DoOnce false))
          (:NewEnumerator4
            (Utilities|FlowControl|DoOnce false
              (:Completed
                (bind _returnvalue_3 (Game|AddComponentbyClass (Variables|Default|GetOwning%20Actor) "/Game/SuperPowers/Invisibility/SC_Invisibility.SC_Invisibility_C" false))
                (CallFunction|AddNewPower _returnvalue_3))))
          (:NewEnumerator5
            (Utilities|FlowControl|DoOnce false
              (:Completed
                (bind _returnvalue_4 (Game|AddComponentbyClass (Variables|Default|GetOwning%20Actor) "/Game/SuperPowers/LazerEyes/SC_LazerEyeComponent.SC_LazerEyeComponent_C" false))
                (CallFunction|AddNewPower _returnvalue_4))))
          (:NewEnumerator6
            (Utilities|FlowControl|DoOnce false)))))
    (:then_2
      (Utilities|IsValid _power_component
        (:Is%20Valid
          (Variables|Default|SetActive%20Power%20Name _power_name)
          (bind _output_get (Variables|Default|SetCurrently%20Active%20Power _power_component))
          (Default|SetasActivePower _output_get true))))))

(fn AddNewPower
  (params (Super%20Power%20Component :type Scene%20Component%20Object%20Reference%20%28by%20ref%29))
  (bind _assc_parent_sub_super_powers_component (Utilities|Casting|CastToSC_ParentSubSuperPowersComponent Super%20Power%20Component)
    (:then
      (bind _returnvalue (Transformation|AttachComponentToComponent _assc_parent_sub_super_powers_component self "None" "SnapToTarget" "SnapToTarget" "SnapToTarget" true))
      (if _returnvalue
        (Utilities|Array|Add (Variables|Default|GetSuper%20Power%20Components) _assc_parent_sub_super_powers_component)
        (Development|PrintString (Utilities|String|Append (Utilities|GetDisplayName Super%20Power%20Component) " Added"))
        (else
          (Development|PrintString (Utilities|String|Append "Error: Could Not Add " (Utilities|GetDisplayName Super%20Power%20Component) " To Super Powers") true true "(R=1.000000,G=0.000000,B=0.000000,A=1.000000)" 1e+01 :!label _label))))
    (:CastFailed
      (goto _label))))

(fn GetSuperPowerbyIndex
  (params (Index :type Integer))
  (bind _super_power_components (Variables|Default|GetSuper%20Power%20Components))
  (bind _output (Utilities|Array|Get(acopy) _super_power_components Index))
  (return _output (Variables|/Game/SuperPowers/ParentPower/SC_ParentSubSuperPowersComponent.SC_ParentSubSuperPowersComponent_C|GetName _output)))